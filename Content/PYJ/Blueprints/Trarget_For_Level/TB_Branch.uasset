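; TB_Branch is a level target actor that spawns a TB_TargetPSpot in front of its CameraRoot on BeginPlay.
; The spot sits a fixed distance from the actor's root along CameraRoot's forward vector, rotated to look back at the root.
; Debug prints show the rotations, and Tick draws a debug line outward from that spot.
; The construction script sets BranchRoot's X offset to half the Cube's X scale.
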(event EventBeginPlay
  (bind _defaultsceneroot (Variables|Default|GetDefaultSceneRoot))
  (bind _cameraroot (Variables|Default|GetCameraRoot))
  (bind _returnvalue (Transformation|GetWorldLocation _defaultsceneroot))
  (bind _returnvalue_2 (Math|Vector|GetForwardVector _cameraroot))
  (bind _returnvalue_3 (* _returnvalue_2 5e+02))
  (bind _returnvalue_4 (+ _returnvalue _returnvalue_3))
  (bind _returnvalue_5 (Math|Rotator|FindLookatRotation _returnvalue_4 _returnvalue))
  (Development|PrintString (Utilities|String|ToString(Rotator) (Math|Conversions|RotationFromXVector _returnvalue_3)) true true "(R=1.000000,G=0.038177,B=0.000000,A=1.000000)" 1e+02)
  (Development|PrintString (Utilities|String|ToString(Rotator) _returnvalue_5) true true "(R=0.000000,G=0.660000,B=1.000000,A=1.000000)" 1e+02)
  (Game|SpawnActorfromClass "/Game/PYJ/Blueprints/Trarget_For_Level/TB_TargetPSpot.TB_TargetPSpot_C" (Math|Transform|MakeTransform _returnvalue_4 _returnvalue_5 "1,1,1") "AlwaysSpawn" 0 0))

(event Collision|EventActorBeginOverlap
  (params (OtherActor :type Actor%20Object%20Reference)))

(event EventTick
  (params (DeltaSeconds :type Float%20%28single-precision%29))
  (bind _defaultsceneroot (Variables|Default|GetDefaultSceneRoot))
  (bind _cameraroot (Variables|Default|GetCameraRoot))
  (bind _returnvalue (Transformation|GetWorldLocation _defaultsceneroot))
  (bind _returnvalue_2 (Math|Vector|GetForwardVector _cameraroot))
  (bind _returnvalue_3 (* _returnvalue_2 5e+02))
  (bind _returnvalue_4 (+ _returnvalue _returnvalue_3))
  (Rendering|Debug|DrawDebugLine :LineStart _returnvalue_4 :LineEnd (+ _returnvalue_4 (* (Math|Vector|GetForwardVector (Variables|Default|GetCameraRoot)) 1e+02)) :Duration 1e+01 :Thickness 1e+01))

(fn ConstructionScript
  (Transformation|SetRelativeLocation (Variables|Default|GetBranchRoot) (Math|Vector|MakeVector (/ (.x (Variables|/Script/Engine.SceneComponent|GetRelativeScale3D (Variables|Default|GetCube))) 2.0) 0.0 0.0) false false))