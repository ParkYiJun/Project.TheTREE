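; TB_GameModeNormal is a game mode Blueprint that starts an "exclamation" identified by a code and is meant to light up its locations.
; StartExclamation stores the code and its table row's HKind through SetForCom, then calls VisibleLocation on each GetHKindArray element.
; GetHKindArray's HKind-to-location Select is unconnected, with no Loc04 entry.
; EndExclamation, BeginPlay, Tick and the construction script are empty.
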(event EventBeginPlay)

(event EventTick
  (params (DeltaSeconds :type Float%20%28single-precision%29)))

(fn ConstructionScript)

(fn StartExclamation
  (params (Code :type Integer))
  (Utilities|SetforCom Code)
  ;[1 1 1] Light On Locs
  (for _array_element (Utilities|GetHKindArray)
    (Default|VisibleLocation _array_element)))

(fn EndExclamation
  (params (NewParam :type Boolean)))