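; TB_PlayerPawn is a player pawn Blueprint that currently holds only controller assignment and facing-direction debug output.
; BeginPlay sets AIControllerClass to TB_PlayerController, then runs a short Delay with nothing after it.
; Each Tick draws a debug line along the DefaultSceneRoot forward vector and prints the rotation derived from that vector.
; ActorBeginOverlap and the construction script are empty.
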(event EventBeginPlay
  (Variables|Default|SetAIControllerClass "/Game/PYJ/Blueprints/Player/TB_PlayerController.TB_PlayerController_C")
  (Utilities|FlowControl|Delay 0.2))

(event Collision|EventActorBeginOverlap
  (params (OtherActor :type Actor%20Object%20Reference)))

(event EventTick
  (params (DeltaSeconds :type Float%20%28single-precision%29))
  (bind _defaultsceneroot (Variables|Default|GetDefaultSceneRoot))
  (bind _returnvalue (Transformation|GetWorldLocation _defaultsceneroot))
  (bind _returnvalue_2 (Math|Vector|GetForwardVector _defaultsceneroot))
  (Rendering|Debug|DrawDebugLine _returnvalue (+ _returnvalue (* _returnvalue_2 1e+02)) "(R=1.000000,G=0.000000,B=0.000000,A=1.000000)" 1.0 5.0)
  (Development|PrintString (Utilities|String|ToString(Rotator) (Math|Conversions|RotationFromXVector _returnvalue_2)) true true "(R=1.000000,G=1.000000,B=0.000000,A=1.000000)" 0.01))

(fn ConstructionScript)