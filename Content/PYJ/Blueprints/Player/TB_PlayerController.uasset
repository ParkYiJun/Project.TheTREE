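; Player controller that classifies touch gestures and converts drags into view move and zoom values.
; On BeginPlay it resets the gesture state and copies the transform of the first TB_TargetPSpot actor.
; Gates and short delays distinguish single, double and long taps, alongside single and dual-finger drags.
; Stored press and release points yield a dominant-axis swipe displacement or two-finger distance change, saved to variables without being applied here.
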(event EventBeginPlay
  (CallFunction|InitVariable)
  (bind _outactors (Actor|GetAllActorsOfClass "/Game/PYJ/Blueprints/Trarget_For_Level/TB_TargetPSpot.TB_TargetPSpot_C"))
  (Development|PrintString (Utilities|String|ToString(Rotator) (.rotation (Transformation|GetActorTransform (Utilities|Array|Get(acopy) _outactors)))) true true "(R=1.000000,G=0.000000,B=0.992903,A=1.000000)" 1e+02)
  (Transformation|SetActorTransform (Math|Transform|MakeTransform (.location (Transformation|GetActorTransform (Utilities|Array|Get(acopy) _outactors))) (.rotation (Transformation|GetActorTransform (Utilities|Array|Get(acopy) _outactors))) (.scale (Transformation|GetActorTransform (Utilities|Array|Get(acopy) _outactors))))))

(event EventTick
  (params (DeltaSeconds :type Float%20%28single-precision%29)))

(event Input|TouchEvents|Touch1
  (params (Key :type Key%20Structure))
  (:Pressed
    (Utilities|IsSingleTap ; Single / Double
      (:Then
        ;[1 1 1] E_Touch: DoubleTap
        (Utilities|FlowControl|Gate true :!label _label
          (:Exit
            (Variables|Default|SetE_Touch "NewEnumerator3"))))
      (:else
        ;[1 1 1] E_Touch: SingleTap, LongSingleTap
        (Variables|Default|SetE_Touch "NewEnumerator1")
        (Utilities|FlowControl|Sequence
          (:then_0
            (goto _label_2 Open))
          (:then_1
            ;[1 1 1] E_Touch: SingleTap (Pass in Time for judging LongSingle-Touch)
            (Utilities|FlowControl|Delay 0.1)
            (goto _label_2 Close))))))
  (:Released
    ;[1 1 1] E_Touch: LongSingleTap
    (Utilities|IsSingleTap
      (:Then
        (Variables|Default|SetE_Touch "NewEnumerator2")
        (Utilities|FlowControl|Gate true :!label _label_2
          (:Exit
            (Variables|Default|SetE_Touch "NewEnumerator1")
            ;[1 1 1] E_Touch: Prepare for DoubleTap
            (Utilities|FlowControl|Sequence
              (:then_0
                (goto _label Open))
              (:then_1
                (Utilities|FlowControl|Delay 0.23)
                (goto _label Close)))))))))

(event Input|TouchEvents|Touch2
  (params (Key :type Key%20Structure))
  ;[1 1 1] E_Touch: DualTapDrag
  (:Pressed
    (Variables|Default|SetE_Touch "NewEnumerator4")))

(event Input|TouchEvents|InputTouch
  (params (Location :type Vector) (FingerIndex :type ETouchIndex%20Enum))
  (:Pressed
    (switch Utilities|FlowControl|Switch|SwitchonETouchIndex FingerIndex
      (:Touch1
        (Utilities|SetSTPressed Location :!label _label))
      (:Touch2
        (goto _label setVec2))))
  (:Released
    (Utilities|IsDragTouch)
    (switch Utilities|FlowControl|Switch|SwitchonETouchIndex FingerIndex
      (:Touch1
        (Utilities|SetSTReleased Location :!label _label_2
          (:Single
            (CallFunction|FViewMove))
          (:Dual
            (CallFunction|FViewZoom))))
      (:Touch2
        (goto _label_2 setVec2))))
  (:Moved
    ;[1 1 1] E_Touch: Single Tap Drag
    (switch Utilities|FlowControl|Switch|SwitchonETouchIndex FingerIndex
      (:Touch1
        (if (Utilities|Enum|NotEqual(Enum) (Variables|Default|GetE_Touch) "NewEnumerator4")
          (Variables|Default|SetE_Touch "NewEnumerator7"))))))

(fn ConstructionScript)

(fn InitVariable
  (Variables|Default|SetE_Touch "NewEnumerator6"))

(fn FViewMove
  (bind _st_pressedt (Variables|Default|GetST_PressedT))
  (bind _st_releasedt (Variables|Default|GetST_ReleasedT))
  (bind (_swipedirection _displacement) (Utilities|SetSwipeDirection (.v1 _st_pressedt) (.v1 _st_releasedt)))
  (switch Utilities|FlowControl|Switch|SwitchonETouchSwipeDirection _swipedirection
    (:Left
      (Variables|Default|SetVV_Displacement (Math|Vector|MakeVector _displacement 0.0 0.0)))
    (:Up
      (Variables|Default|SetVV_Displacement (Math|Vector|MakeVector 0.0 _displacement 0.0))))
  (return))

(fn FViewZoom
  (Variables|Default|SetVF_ZoomDis (- (Utilities|BetweenVecs (Variables|Default|GetST_ReleasedT)) (Utilities|BetweenVecs (Variables|Default|GetST_PressedT)))))