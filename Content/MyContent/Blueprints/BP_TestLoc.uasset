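; BP_TestLoc is a test location actor that looks up an animal's habitat data and can reveal a point light through VisibleLocation.
; FindLocSM reads the DT_AnimalAsset row for an animal code, stores its Habitat in TestMesh and reports success.
; SetLocSM applies GetGraphic to the LocLoading mesh, but GetGraphic's conversion node is unconnected.
; Light activation toggles a touch-enter gate that drives nothing, and ActiveLocation is empty.
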(event OnComponentActivated(PointLight)
  (params (Component :type Actor%20Component%20Object%20Reference) (bReset :type Boolean))
  (Utilities|FlowControl|Gate true) ; enters at Open
)

(event OnComponentDeactivated(PointLight)
  (params (Component :type Actor%20Component%20Object%20Reference))
  (Utilities|FlowControl|Gate true) ; enters at Close
)

(event Custom|VisibleLocation
  (Rendering|SetVisibility (Variables|Default|GetPointLight) true false))

(event EventActorOnInputTouchEnter
  (params (FingerIndex :type ETouchIndex%20Enum :default "Touch1"))
  (Utilities|FlowControl|Gate true))

(fn ConstructionScript)

(fn ActiveLocation)

(fn FindLocSM
  (params (AnimalCode :type Integer))
  (bind _returnvalue (Utilities|GetDataTableRow "/Game/PYJ/Blueprints/Animal/DataTable/DT_AnimalAsset.DT_AnimalAsset" (Utilities|String|StringToName (Utilities|String|ToString(Integer) AnimalCode)))
    (:then
      (Variables|Default|SetTestMesh (.habitat _returnvalue))
      (return true))
    (:RowNotFound
      (return false))))

(fn SetLocSM
  (Components|StaticMesh|SetStaticMesh (Variables|Default|GetLocLoading) (Utilities|GetGraphic)))